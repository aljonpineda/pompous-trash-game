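; BP_NoAimAssistRicochetHat is a spinning thrown-hat projectile that ricochets off surfaces and is destroyed when it overlaps a pawn.
; BeginPlay applies the launch impulse and stores a camera-forward version for later reflections.
; Hits on one custom channel reverse the launch impulse, or enable gravity after a bounce; the other channel mirrors the current impulse by hit normal.
; Each bounce shakes the camera and toggles physics simulation to discard built-in collision response.
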(event `self.ReceiveBeginPlay`
  (bind _initialimpulse (`self.InitialImpulse`))
  (`PrimitiveComponent.AddImpulse` (`self.CollisionComponent`) _initialimpulse "None" false)
  (bind _impulse (`self.Get Straightened Impulse` _initialimpulse))
  (set `self.CurrentImpulse` _impulse))

(event `self.CollisionComponent.OnComponentBeginOverlap`
  (params (OverlappedComponent :type "PrimitiveComponent Object Reference") (OtherActor :type "Actor Object Reference") (OtherComp :type "PrimitiveComponent Object Reference") (OtherBodyIndex :type Integer) (bFromSweep :type Boolean) (SweepResult :type "HitResult Structure (by ref)"))
  ;[0 0 0] Destroy hat when it overlaps with the player
  (if (`|EnumEquality` (`PrimitiveComponent.GetCollisionObjectType` OtherComp) "ECC_Pawn")
    (`self.K2_DestroyActor`)))

(event `self.CollisionComponent.OnComponentHit`
  (params (HitComponent :type "PrimitiveComponent Object Reference") (OtherActor :type "Actor Object Reference") (OtherComp :type "PrimitiveComponent Object Reference") (NormalImpulse :type "Vector Structure") (Hit :type "HitResult Structure (by ref)"))
  (bind _returnvalue (`PrimitiveComponent.GetCollisionObjectType` OtherComp))
  (if (`|EnumEquality` _returnvalue "ECC_GameTraceChannel1")
    (if (`self.HasBounced`)
      (if (not (`self.IsGravityEnabled`))
        (`self.Prepare Bounce`)
        (`PrimitiveComponent.SetEnableGravity` (`self.CollisionComponent`) true)
        (set `self.IsGravityEnabled` true))
      (else
        (`self.Prepare Bounce`)
        (set `self.CurrentImpulse` (`KismetMathLibrary.NegateVector` (`self.InitialImpulse`)))
        (`PrimitiveComponent.AddImpulse` (`self.CollisionComponent`) (`self.CurrentImpulse`) "None" false :!label _label)
        (set `self.HasBounced` true)))
    (elif (`|EnumEquality` _returnvalue "ECC_GameTraceChannel2")
      (`self.Prepare Bounce`)
      (set `self.CurrentImpulse` (`KismetMathLibrary.MirrorVectorByNormal` (`self.CurrentImpulse`) (`.Normal` (`GameplayStatics.BreakHitResult` Hit))))
      (goto _label))))

(event `self.ReceiveTick`
  (params (DeltaSeconds :type "Float (single-precision)"))
  (`self.K2_AddActorLocalRotation` (* (`self.DeltaRotation`) DeltaSeconds)))

(fn `Add Camera Shake`
  (`GameplayStatics.PlayWorldCameraShake` "/Game/PompousTrashGame/Blueprints/BP_BounceCameraShake.BP_BounceCameraShake_C" (0.0 0.0 0.0) 0.0 5000.0 0.5))

(fn `Get Signed Angle Between Vectors`
  (params (A :type "Vector Structure") (B :type "Vector Structure") (Up :type "Vector Structure"))
  (returns (Angle :type "Float (double-precision)"))
  (bind _returnvalue (`KismetMathLibrary.Normal` B))
  (bind _returnvalue_2 (`KismetMathLibrary.Normal` A))
  (bind _returnvalue_3 (`KismetMathLibrary.DegAcos` (`KismetMathLibrary.Dot_VectorVector` _returnvalue_2 _returnvalue)))
  (if (< (`KismetMathLibrary.Dot_VectorVector` Up (`KismetMathLibrary.Cross_VectorVector` _returnvalue_2 _returnvalue)) 0.0)
    (bind _result (`/Engine/EditorBlueprintResources/StandardMacros.NegateFloat` _returnvalue_3)
      (:`  `
        (return _result)))
    (else
      (return _returnvalue_3))))

(fn `Get Straightened Impulse`
  (params (InitialImpulse :type "Vector Structure"))
  (returns (Impulse :type "Vector Structure"))
  (return (* (`KismetMathLibrary.VSize` InitialImpulse) (`self.GetActorForwardVector` (`GameplayStatics.GetPlayerCameraManager` 0)))))

(fn `Prepare Bounce`
  (`self.Add Camera Shake`)
  (`self.Restart Physics`) ; Turn physics off and on to remove built-in collision mechanics
)

(fn `Restart Physics`
  (bind _collisioncomponent (`self.CollisionComponent`))
  (`PrimitiveComponent.SetSimulatePhysics` _collisioncomponent false)
  (`PrimitiveComponent.SetSimulatePhysics` _collisioncomponent true))

(fn `Round to Nearest`
  (params (Value :type "Float (double-precision)") (Nearest :type Integer))
  (returns (Result :type Integer))
  (return (* (`KismetMathLibrary.Round` (`KismetMathLibrary.SafeDivide` Value (`KismetMathLibrary.Conv_IntToDouble` Nearest))) Nearest)))

(fn `UserConstructionScript`)