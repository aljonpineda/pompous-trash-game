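; Actor component that rotates its owning wall by a target offset when a linked button is hit.
; The first rotation creates two corner Niagara smoke effects, which later rotations restart.
; Tick lerps from the starting rotation at a set speed, then snaps to the end and plays a world camera shake.
; Persistent walls reset to rotate again from the new orientation; otherwise the component destroys itself.
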(event `self.ReceiveBeginPlay`
  (set `self.InitialRotation` (`Actor.K2_GetActorRotation` (`self.GetOwner`)))
  (add `/Game/PompousTrashGame/Blueprints/BP_Button.OnButtonHit` (`self.ButtonHit`) (delegate `OnButtonHit`)))

(event `Rotate`
  (bind _returnvalue (`self.GetOwner`))
  (if (`self.IsNiagaraInitialized`)
    (if (not (`self.IsRotating`))
      (`NiagaraComponent.ReinitializeSystem` (stale _returnvalue_2))
      (`NiagaraComponent.ReinitializeSystem` (stale _returnvalue_3))
      (set `self.IsRotating` true :!label _label))
    (else
      (bind _returnvalue_2 (`|AddComponentByClass` _returnvalue "/Script/Niagara.NiagaraComponent" false (`KismetMathLibrary.MakeTransform` (`self.FirstCorner`))))
      (`NiagaraComponent.SetAsset` _returnvalue_2 "/Game/PompousTrashGame/FX/NS_MovingWallSmoke.NS_MovingWallSmoke" true)
      (bind _returnvalue_3 (`|AddComponentByClass` _returnvalue "/Script/Niagara.NiagaraComponent" false (`KismetMathLibrary.MakeTransform` (`self.SecondCorner`))))
      (`NiagaraComponent.SetAsset` _returnvalue_3 "/Game/PompousTrashGame/FX/NS_MovingWallSmoke.NS_MovingWallSmoke" true)
      (set `self.IsNiagaraInitialized` true)
      (goto _label))))

(event `OnButtonHit`
  (`self.Rotate`))

(event `self.ReceiveTick`
  (params (DeltaSeconds :type "Float (single-precision)"))
  (bind _returnvalue (`self.GetOwner`))
  (bind _initialrotation (`self.InitialRotation`))
  (bind _returnvalue_2 (`KismetMathLibrary.RLerp` _initialrotation (`KismetMathLibrary.MakeRotator` (+ (.roll _initialrotation) (.roll (`self.TargetRotation`))) (+ (.pitch _initialrotation) (.pitch (`self.TargetRotation`))) (+ (.yaw _initialrotation) (.yaw (`self.TargetRotation`)))) (`self.Alpha`)))
  (if (`self.IsRotating`)
    (bind _output_get (set `self.Alpha` (+ (* DeltaSeconds (`self.RotationSpeed`)) (`self.Alpha`))))
    (if (<= _output_get 1.0)
      (`Actor.K2_SetActorRotation` _returnvalue _returnvalue_2 false)
      (else
        (set `self.Alpha` 1.0)
        (`Actor.K2_SetActorRotation` _returnvalue _returnvalue_2 false) ; Correct final rotation
        (`GameplayStatics.PlayWorldCameraShake` "/Game/PompousTrashGame/Blueprints/BP_WallCameraShake.BP_WallCameraShake_C" (`Actor.K2_GetActorLocation` _returnvalue) 0.0 1000.0 0.1)
        (if (`self.IsPersistent`)
          (set `self.Alpha` 0.0)
          (set `self.IsRotating` false)
          (set `self.InitialRotation` (`Actor.K2_GetActorRotation` (`self.GetOwner`)))
          (else
            (`self.K2_DestroyComponent`)))))))