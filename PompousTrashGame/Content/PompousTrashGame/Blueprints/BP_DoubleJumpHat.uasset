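; BP_DoubleJumpHat is a physics-driven hat actor that destroys itself when a Pawn-type component overlaps it.
; On BeginPlay, its collision component receives an impulse built from InitialImpulse and ImpulseMultiplier, rotated by the actor's rotation so the launch follows its facing.
; A RestartPhysics function toggles physics simulation off and on.
; No double-jump logic appears in this Blueprint.
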(event `self.CollisionComponent.OnComponentBeginOverlap`
  (params (OverlappedComponent :type "PrimitiveComponent Object Reference") (OtherActor :type "Actor Object Reference") (OtherComp :type "PrimitiveComponent Object Reference") (OtherBodyIndex :type Integer) (bFromSweep :type Boolean) (SweepResult :type "HitResult Structure (by ref)"))
  ;[0 0 0] Destroy hat when it overlaps with the player
  (if (`|EnumEquality` (`PrimitiveComponent.GetCollisionObjectType` OtherComp) "ECC_Pawn")
    (`self.K2_DestroyActor`)))

(event `self.ReceiveBeginPlay`
  (`PrimitiveComponent.AddImpulse` (`self.CollisionComponent`) (`KismetMathLibrary.GreaterGreater_VectorRotator` (* (`self.ImpulseMultiplier`) (`self.InitialImpulse`)) (`self.K2_GetActorRotation`)) "None" false))

(fn `Restart Physics`
  (bind _collisioncomponent (`self.CollisionComponent`))
  (`PrimitiveComponent.SetSimulatePhysics` _collisioncomponent false)
  (`PrimitiveComponent.SetSimulatePhysics` _collisioncomponent true))

(fn `UserConstructionScript`)