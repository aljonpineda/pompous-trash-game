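; BP_PlatformHat is a physics-driven hat projectile that turns into a BP_Platform where it lands.
; On BeginPlay it applies its impulse, then stores a copy redirected along the camera's forward vector.
; Hitting either of two custom object channels spawns a platform offset along the surface normal, replaces the player's previous one and destroys the hat; overlapping a Pawn just destroys it.
; Physics-restart, signed-angle and rounding helpers are defined but not called here.
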(event `self.ReceiveBeginPlay`
  (bind _currentimpulse (`self.CurrentImpulse`))
  (`PrimitiveComponent.AddImpulse` (`self.CollisionComponent`) _currentimpulse "None" false)
  (bind _impulse (`self.Get Straightened Impulse` _currentimpulse))
  (set `self.CurrentImpulse` _impulse))

(event `self.CollisionComponent.OnComponentBeginOverlap`
  (params (OverlappedComponent :type "PrimitiveComponent Object Reference") (OtherActor :type "Actor Object Reference") (OtherComp :type "PrimitiveComponent Object Reference") (OtherBodyIndex :type Integer) (bFromSweep :type Boolean) (SweepResult :type "HitResult Structure (by ref)"))
  ;[0 0 0] Destroy hat when it overlaps with the player
  (if (`|EnumEquality` (`PrimitiveComponent.GetCollisionObjectType` OtherComp) "ECC_Pawn")
    (`self.K2_DestroyActor`)))

(event `self.CollisionComponent.OnComponentHit`
  (params (HitComponent :type "PrimitiveComponent Object Reference") (OtherActor :type "Actor Object Reference") (OtherComp :type "PrimitiveComponent Object Reference") (NormalImpulse :type "Vector Structure") (Hit :type "HitResult Structure (by ref)"))
  (bind _returnvalue (`PrimitiveComponent.GetCollisionObjectType` OtherComp))
  (bind (_bblockinghit _binitialoverlap _time _distance _location _impactpoint _normal) (`GameplayStatics.BreakHitResult` Hit))
  (bind _player (`self.Player`))
  (bind _currentplatform (`/Game/PompousTrashGame/Blueprints/BP_PompousCharacter.CurrentPlatform` _player))
  (if (or (`|EnumEquality` _returnvalue "ECC_GameTraceChannel1") (`|EnumEquality` _returnvalue "ECC_GameTraceChannel2"))
    (bind _returnvalue_2 (`|SpawnActorFromClass` "/Game/PompousTrashGame/Blueprints/BP_Platform.BP_Platform_C" (`KismetMathLibrary.MakeTransform` (+ _location (* _normal (`self.PlatformOffset`))) (struct :`Yaw` 90.0)) "AlwaysSpawn" "MultiplyWithRoot" null null))
    (`/Engine/EditorBlueprintResources/StandardMacros.IsValid` _currentplatform
      (:`Is Valid`
        (`self.K2_DestroyActor` _currentplatform))
      (:`Is Not Valid`
        _))
    (set `/Game/PompousTrashGame/Blueprints/BP_PompousCharacter.CurrentPlatform` _returnvalue_2 _player)
    (`self.K2_DestroyActor`)))

(fn `Get Signed Angle Between Vectors`
  (params (A :type "Vector Structure") (B :type "Vector Structure") (Up :type "Vector Structure"))
  (returns (Angle :type "Float (double-precision)"))
  (bind _returnvalue (`KismetMathLibrary.Normal` B))
  (bind _returnvalue_2 (`KismetMathLibrary.Normal` A))
  (bind _returnvalue_3 (`KismetMathLibrary.DegAcos` (`KismetMathLibrary.Dot_VectorVector` _returnvalue_2 _returnvalue)))
  (if (< (`KismetMathLibrary.Dot_VectorVector` Up (`KismetMathLibrary.Cross_VectorVector` _returnvalue_2 _returnvalue)) 0.0)
    (bind _result (`/Engine/EditorBlueprintResources/StandardMacros.NegateFloat` _returnvalue_3)
      (:`  `
        (return _result)))
    (else
      (return _returnvalue_3))))

(fn `Get Straightened Impulse`
  (params (InitialImpulse :type "Vector Structure"))
  (returns (Impulse :type "Vector Structure"))
  (return (* (`KismetMathLibrary.VSize` InitialImpulse) (`self.GetActorForwardVector` (`GameplayStatics.GetPlayerCameraManager` 0)))))

(fn `Restart Physics`
  (bind _collisioncomponent (`self.CollisionComponent`))
  (`PrimitiveComponent.SetSimulatePhysics` _collisioncomponent false)
  (`PrimitiveComponent.SetSimulatePhysics` _collisioncomponent true))

(fn `Round to Nearest`
  (params (Value :type "Float (double-precision)") (Nearest :type Integer))
  (returns (Result :type Integer))
  (return (* (`KismetMathLibrary.Round` (`KismetMathLibrary.SafeDivide` Value (`KismetMathLibrary.Conv_IntToDouble` Nearest))) Nearest)))

(fn `UserConstructionScript`)