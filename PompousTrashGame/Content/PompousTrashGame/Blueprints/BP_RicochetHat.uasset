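; BP_RicochetHat is a physics-driven hat projectile that launches along its rotation, bounces off surfaces and is destroyed on overlapping a pawn.
; GameTraceChannel1 hits reverse it if it has not bounced yet, otherwise enable gravity.
; GameTraceChannel2 hits always reflect it, snapping the angle from the normal to set intervals around the hit actor's up axis.
; Both restart physics to cancel built-in collision response before reapplying impulses.
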(event `self.CollisionComponent.OnComponentBeginOverlap`
  (params (OverlappedComponent :type "PrimitiveComponent Object Reference") (OtherActor :type "Actor Object Reference") (OtherComp :type "PrimitiveComponent Object Reference") (OtherBodyIndex :type Integer) (bFromSweep :type Boolean) (SweepResult :type "HitResult Structure (by ref)"))
  ;[0 0 0] Destroy hat when it overlaps with the player
  (if (`|EnumEquality` (`PrimitiveComponent.GetCollisionObjectType` OtherComp) "ECC_Pawn")
    (`self.K2_DestroyActor`)))

(event `self.ReceiveBeginPlay`
  (bind _output_get (set `self.CurrentImpulse` (`KismetMathLibrary.GreaterGreater_VectorRotator` (* (`self.ImpulseMultiplier`) (`self.InitialImpulse`)) (`self.K2_GetActorRotation`))))
  (`PrimitiveComponent.AddImpulse` (`self.CollisionComponent`) _output_get "None" false))

(event `self.CollisionComponent.OnComponentHit`
  (params (HitComponent :type "PrimitiveComponent Object Reference") (OtherActor :type "Actor Object Reference") (OtherComp :type "PrimitiveComponent Object Reference") (NormalImpulse :type "Vector Structure") (Hit :type "HitResult Structure (by ref)"))
  (bind _returnvalue (`PrimitiveComponent.GetCollisionObjectType` OtherComp))
  (bind _returnvalue_2 (`self.GetActorUpVector` OtherActor))
  (bind (_bblockinghit _binitialoverlap _time _distance _location _impactpoint _normal) (`GameplayStatics.BreakHitResult` Hit))
  (bind _returnvalue_3 (`KismetMathLibrary.MirrorVectorByNormal` (`self.CurrentImpulse`) _normal))
  (if (`|EnumEquality` _returnvalue "ECC_GameTraceChannel1")
    (`self.Restart Physics`) ; Turn physics off and on to remove built-in collision mechanics
    (if (`self.HasBounced`)
      (`PrimitiveComponent.SetEnableGravity` (`self.CollisionComponent`) true)
      (else
        (bind _output_get (set `self.CurrentImpulse` (`KismetMathLibrary.NegateVector` (`self.CurrentImpulse`))))
        (`PrimitiveComponent.AddImpulse` (`self.CollisionComponent`) _output_get "None" false)
        (set `self.HasBounced` true :!label _label)))
    (elif (`|EnumEquality` _returnvalue "ECC_GameTraceChannel2")
      (`self.Restart Physics`) ; Turn physics off and on to remove built-in collision mechanics
      (bind _angle (`self.Get Signed Angle Between Vectors` _normal _returnvalue_3 _returnvalue_2))
      (`KismetSystemLibrary.PrintString` (`KismetStringLibrary.Conv_DoubleToString` _angle))
      (bind _result (`self.Round to Nearest` _angle (`self.AngleIntervalSize`)))
      (`KismetSystemLibrary.PrintString` (`KismetStringLibrary.Conv_IntToString` _result))
      (bind _output_get_2 (set `self.CurrentImpulse` (`KismetMathLibrary.RotateAngleAxis` _returnvalue_3 (- (`KismetMathLibrary.Clamp` _result -89 89) _angle) _returnvalue_2)))
      (`PrimitiveComponent.AddImpulse` (`self.CollisionComponent`) _output_get_2 "None" false)
      (goto _label))))

(fn `Get Signed Angle Between Vectors`
  (params (A :type "Vector Structure") (B :type "Vector Structure") (Up :type "Vector Structure"))
  (returns (Angle :type "Float (double-precision)"))
  (bind _returnvalue (`KismetMathLibrary.Normal` B))
  (bind _returnvalue_2 (`KismetMathLibrary.Normal` A))
  (bind _returnvalue_3 (`KismetMathLibrary.DegAcos` (`KismetMathLibrary.Dot_VectorVector` _returnvalue_2 _returnvalue)))
  (if (< (`KismetMathLibrary.Dot_VectorVector` Up (`KismetMathLibrary.Cross_VectorVector` _returnvalue_2 _returnvalue)) 0.0)
    (bind _result (`/Engine/EditorBlueprintResources/StandardMacros.NegateFloat` _returnvalue_3)
      (:`  `
        (return _result)))
    (else
      (return _returnvalue_3))))

(fn `Restart Physics`
  (bind _collisioncomponent (`self.CollisionComponent`))
  (`PrimitiveComponent.SetSimulatePhysics` _collisioncomponent false)
  (`PrimitiveComponent.SetSimulatePhysics` _collisioncomponent true))

(fn `Round to Nearest`
  (params (Value :type "Float (double-precision)") (Nearest :type Integer))
  (returns (Result :type Integer))
  (return (* (`KismetMathLibrary.Round` (`KismetMathLibrary.SafeDivide` Value (`KismetMathLibrary.Conv_IntToDouble` Nearest))) Nearest)))

(fn `UserConstructionScript`)