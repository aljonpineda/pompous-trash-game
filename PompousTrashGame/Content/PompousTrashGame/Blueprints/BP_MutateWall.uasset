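; BP_MutateWall is a component that transforms its owning static mesh actor when a linked button is hit.
; On BeginPlay it binds to the OnButtonHit dispatcher of its ButtonHit reference, which triggers Mutate.
; Mutate switches the mesh to a custom collision object channel, applies a white material, then destroys the component, making the change one-shot.
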(event `self.ReceiveBeginPlay`
  (add `/Game/PompousTrashGame/Blueprints/BP_Button.OnButtonHit` (`self.ButtonHit`) (delegate `OnButtonHit`)))

(event `OnButtonHit`
  (`self.Mutate`))

(event `Mutate`
  (bind _asstatic_mesh_actor (cast `StaticMeshActor` (`self.GetOwner`)))
  (bind _staticmeshcomponent (`StaticMeshActor.StaticMeshComponent` _asstatic_mesh_actor))
  (`PrimitiveComponent.SetCollisionObjectType` _staticmeshcomponent "ECC_GameTraceChannel2")
  (`PrimitiveComponent.SetMaterial` _staticmeshcomponent 0 "/Game/PompousTrashGame/Materials/M_White.M_White")
  (`self.K2_DestroyComponent`))