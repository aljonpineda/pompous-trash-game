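; BP_Hat is a physics-driven hat projectile that launches itself on spawn and is destroyed when it overlaps a Pawn, intended as the player.
; BeginPlay applies a scaled initial impulse rotated to the actor's facing.
; Each hit toggles physics simulation to clear motion, then re-applies an impulse by collision channel.
; GameTraceChannel1 hits reverse the rotated launch impulse, while GameTraceChannel2 hits mirror the current impulse around the surface normal.
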(event `self.CollisionComponent.OnComponentBeginOverlap`
  (params (OverlappedComponent :type "PrimitiveComponent Object Reference") (OtherActor :type "Actor Object Reference") (OtherComp :type "PrimitiveComponent Object Reference") (OtherBodyIndex :type Integer) (bFromSweep :type Boolean) (SweepResult :type "HitResult Structure (by ref)"))
  ;[0 0 0] Destroy hat when it overlaps with the player
  (if (`|EnumEquality` (`PrimitiveComponent.GetCollisionObjectType` OtherComp) "ECC_Pawn")
    (`self.K2_DestroyActor`)))

(event `self.CollisionComponent.OnComponentHit`
  (params (HitComponent :type "PrimitiveComponent Object Reference") (OtherActor :type "Actor Object Reference") (OtherComp :type "PrimitiveComponent Object Reference") (NormalImpulse :type "Vector Structure") (Hit :type "HitResult Structure (by ref)"))
  (bind _returnvalue (`PrimitiveComponent.GetCollisionObjectType` OtherComp))
  (`self.Restart Physics`)
  (if (`|EnumEquality` _returnvalue "ECC_GameTraceChannel1")
    (bind _output_get (set `self.CurrentImpulse` (`KismetMathLibrary.NegateVector` (`KismetMathLibrary.GreaterGreater_VectorRotator` (* (`self.ImpulseMultiplier`) (`self.InitialImpulse`)) (`self.K2_GetActorRotation`)))))
    (`PrimitiveComponent.AddImpulse` (`self.CollisionComponent`) _output_get "None" false)
    (elif (`|EnumEquality` _returnvalue "ECC_GameTraceChannel2")
      (bind _output_get_2 (set `self.CurrentImpulse` (`KismetMathLibrary.MirrorVectorByNormal` (`self.CurrentImpulse`) (`.Normal` (`GameplayStatics.BreakHitResult` Hit)))))
      (`PrimitiveComponent.AddImpulse` (`self.CollisionComponent`) _output_get_2 "None" false))))

(event `self.ReceiveBeginPlay`
  (bind _output_get (set `self.CurrentImpulse` (`KismetMathLibrary.GreaterGreater_VectorRotator` (* (`self.ImpulseMultiplier`) (`self.InitialImpulse`)) (`self.K2_GetActorRotation`))))
  (`PrimitiveComponent.AddImpulse` (`self.CollisionComponent`) _output_get "None" false))

(fn `Restart Physics`
  (bind _collisioncomponent (`self.CollisionComponent`))
  (`PrimitiveComponent.SetSimulatePhysics` _collisioncomponent false)
  (`PrimitiveComponent.SetSimulatePhysics` _collisioncomponent true))

(fn `UserConstructionScript`)