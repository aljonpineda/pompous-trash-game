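; BP_TranslateWall is a component that slides its owning actor, by name a wall, along an offset when a button is hit.
; It records the owner's start location on BeginPlay and binds to the button's hit event, which starts the shift.
; Tick then lerps the location toward start plus ShiftVector at LerpSpeed, without sweeping.
; Once alpha exceeds one, the component destroys itself, making the move one-way.
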(event `self.ReceiveBeginPlay`
  (set `self.StartLocation` (`Actor.K2_GetActorLocation` (`self.GetOwner`)))
  (add `/Game/PompousTrashGame/Blueprints/BP_Button.OnButtonHit` (`self.ButtonHit`) (delegate `OnButtonHit`)))

(event `OnButtonHit`
  (`self.Shift`))

(event `Shift`
  (set `self.IsShifting` true))

(event `self.ReceiveTick`
  (params (DeltaSeconds :type "Float (single-precision)"))
  (bind _startlocation (`self.StartLocation`))
  (if (`self.IsShifting`)
    (bind _output_get (set `self.Alpha` (+ (* DeltaSeconds (`self.LerpSpeed`)) (`self.Alpha`))))
    (if (<= _output_get 1.0)
      (`Actor.K2_SetActorLocation` (`self.GetOwner`) (`KismetMathLibrary.VLerp` _startlocation (+ _startlocation (`self.ShiftVector`)) (`self.Alpha`)) false false)
      (else
        (`self.K2_DestroyComponent`)))))